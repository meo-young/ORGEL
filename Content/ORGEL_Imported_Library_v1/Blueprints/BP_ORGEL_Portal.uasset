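; BP_ORGEL_Portal is a wall segment that either shows a framed two-leaf sliding door or a solid wall, chosen by HasDoor.
; Tick moves OpenAmount toward TargetOpen at constant speed, and ApplyDoorState slides the pivots apart and switches visibility and collision, also running at construction and BeginPlay.
; Open, Close and Toggle pass the target to an optional LinkedDoor through SetTargetOpenOnly, which forwards no further, while SetOpenAmount snaps instantly.
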(event EventBeginPlay
  (CallFunction|ApplyDoorState))

(event Collision|EventActorBeginOverlap
  (params (OtherActor :type Actor%20Object%20Reference)))

(event EventTick
  (params (DeltaSeconds :type Float%20%28single-precision%29))
  (Variables|Default|SetOpenAmount (Math|Interpolation|FInterptoConstant (Variables|Default|GetOpenAmount) (Variables|Default|GetTargetOpen) DeltaSeconds (Variables|Default|GetOpenSpeed)))
  (CallFunction|ApplyDoorState))

(fn ConstructionScript
  (CallFunction|ApplyDoorState))

(fn ApplyDoorState
  (Transformation|SetRelativeLocation (Variables|Default|GetLeftPivot) (Math|Vector|MakeVector (* (Variables|Default|GetOpenAmount) -175.0) 0.0 0.0) false false)
  (Transformation|SetRelativeLocation (Variables|Default|GetRightPivot) (Math|Vector|MakeVector (* (Variables|Default|GetOpenAmount) 175.0) 0.0 0.0) false false)
  (Rendering|SetVisibility (Variables|Default|GetLeftPivot) (Variables|Default|GetHasDoor) true)
  (Rendering|SetVisibility (Variables|Default|GetRightPivot) (Variables|Default|GetHasDoor) true)
  (Rendering|SetVisibility (Variables|Default|GetFrameRoot) (Variables|Default|GetHasDoor) true)
  (Rendering|SetVisibility (Variables|Default|GetWallRoot) (not (Variables|Default|GetHasDoor)) true)
  (if (Variables|Default|GetHasDoor)
    (Collision|SetCollisionEnabled (Variables|Default|GetLeftCollision) "QueryAndPhysics")
    (Collision|SetCollisionEnabled (Variables|Default|GetRightCollision) "QueryAndPhysics")
    (Collision|SetCollisionEnabled (Variables|Default|GetWallCollision) "NoCollision")
    (Collision|SetCollisionEnabled (Variables|Default|GetAuxCollision0) "QueryAndPhysics")
    (Collision|SetCollisionEnabled (Variables|Default|GetAuxCollision1) "QueryAndPhysics")
    (Collision|SetCollisionEnabled (Variables|Default|GetAuxCollision2) "QueryAndPhysics")
    (Collision|SetCollisionEnabled (Variables|Default|GetAuxCollision3) "QueryAndPhysics")
    (Collision|SetCollisionEnabled (Variables|Default|GetAuxCollision4) "QueryAndPhysics")
    (else
      (Collision|SetCollisionEnabled (Variables|Default|GetLeftCollision) "NoCollision")
      (Collision|SetCollisionEnabled (Variables|Default|GetRightCollision) "NoCollision")
      (Collision|SetCollisionEnabled (Variables|Default|GetWallCollision) "QueryAndPhysics")
      (Collision|SetCollisionEnabled (Variables|Default|GetAuxCollision0) "NoCollision")
      (Collision|SetCollisionEnabled (Variables|Default|GetAuxCollision1) "NoCollision")
      (Collision|SetCollisionEnabled (Variables|Default|GetAuxCollision2) "NoCollision")
      (Collision|SetCollisionEnabled (Variables|Default|GetAuxCollision3) "NoCollision")
      (Collision|SetCollisionEnabled (Variables|Default|GetAuxCollision4) "NoCollision"))))

(fn SetOpenAmount
  (params (Amount :type Float%20%28double-precision%29))
  (bind _returnvalue (Math|Float|Clamp(Float) Amount 0.0 1.0))
  (Variables|Default|SetOpenAmount _returnvalue)
  (Variables|Default|SetTargetOpen _returnvalue)
  (CallFunction|ApplyDoorState))

(fn SetTargetOpenOnly
  (params (Amount :type Float%20%28double-precision%29))
  (Variables|Default|SetTargetOpen Amount))

(fn OpenDoor
  (bind _linkeddoor (Variables|Default|GetLinkedDoor))
  (Variables|Default|SetTargetOpen 1.0)
  (if (Utilities|IsValid _linkeddoor)
    (CallFunction|SetTargetOpenOnly _linkeddoor (Variables|Default|GetTargetOpen))))

(fn CloseDoor
  (bind _linkeddoor (Variables|Default|GetLinkedDoor))
  (Variables|Default|SetTargetOpen 0.0)
  (if (Utilities|IsValid _linkeddoor)
    (CallFunction|SetTargetOpenOnly _linkeddoor (Variables|Default|GetTargetOpen))))

(fn ToggleDoor
  (bind _linkeddoor (Variables|Default|GetLinkedDoor))
  (Variables|Default|SetTargetOpen (- 1.0 (Variables|Default|GetTargetOpen)))
  (if (Utilities|IsValid _linkeddoor)
    (CallFunction|SetTargetOpenOnly _linkeddoor (Variables|Default|GetTargetOpen))))